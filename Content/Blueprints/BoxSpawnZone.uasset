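; BoxSpawnZone is a spawn zone Blueprint that adds child actors, apparently boxes, at random points inside its Box component's bounds.
; SpawnBox runs a single-iteration loop that adds one child actor component at a random relative transform built from the Box's location and extent.
; The construction script calls SpawnBox, and BeginPlay starts a short one-shot timer whose SpawnNormalBox event calls it again.
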(event `self.ReceiveBeginPlay`
  (`KismetSystemLibrary.K2_SetTimerDelegate` (delegate `SpawnNormalBox`) 2.4))

(event `SpawnNormalBox`
  (`self.SpawnBox`))

(fn `SpawnBox`
  (bind _box (`self.Box`))
  (for _ (range 1)
    (`AddComponent|NODE_AddChildActorComponent-0` :`RelativeTransform` (`KismetMathLibrary.Conv_VectorToTransform` (`KismetMathLibrary.RandomPointInBoundingBox` (`SceneComponent.RelativeLocation` _box) (`BoxComponent.BoxExtent` _box))))))

(fn `UserConstructionScript`
  (switch `int` 0
    (:`Default`
      (`self.SpawnBox`))))